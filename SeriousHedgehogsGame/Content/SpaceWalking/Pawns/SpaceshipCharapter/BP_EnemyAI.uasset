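; Enemy spaceship AI pawn that heads for its road point until it detects the player's spaceship, then chases it.
; Tick drives AIMoveTo toward either target, with PlayerDetected toggled by the outer Sphere's overlaps through paired DoOnce gates.
; During the chase, a DoOnce-gated random roll can trigger a delayed, temporary speed boost with Bust effects.
; Player overlap with Sphere1 opens the level named in LevelToOpenIfOverlap.
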(event OnComponentBeginOverlap(Sphere)
  (params (OverlappedComponent :type Primitive%20Component%20Object%20Reference) (OtherActor :type Actor%20Object%20Reference) (OtherComp :type Primitive%20Component%20Object%20Reference) (OtherBodyIndex :type Integer) (bFromSweep :type Boolean) (SweepResult :type Hit%20Result%20Structure%20%28by%20ref%29))
  (if (not (or (== OtherActor self) (== OtherActor "BP_EnemyAI")))
    (Utilities|Casting|CastToBP_SpaceshipCharacter OtherActor)
    (Utilities|FlowControl|Sequence
      (:then_0
        (Utilities|FlowControl|DoOnce false
          (:Completed
            (Variables|Default|SetPlayerDetected true))))
      (:then_1
        (Utilities|FlowControl|DoOnce false) ; enters at Reset
      ))))

(event OnComponentEndOverlap(Sphere)
  (params (OverlappedComponent :type Primitive%20Component%20Object%20Reference) (OtherActor :type Actor%20Object%20Reference) (OtherComp :type Primitive%20Component%20Object%20Reference) (OtherBodyIndex :type Integer))
  (if (not (or (== OtherActor self) (== OtherActor "BP_EnemyAI")))
    (Utilities|Casting|CastToBP_SpaceshipCharacter OtherActor)
    (Utilities|FlowControl|Sequence
      (:then_0
        (Utilities|FlowControl|DoOnce false
          (:Completed
            (Variables|Default|SetPlayerDetected false))))
      (:then_1
        (Utilities|FlowControl|DoOnce false) ; enters at Reset
      ))))

(event OnComponentBeginOverlap(Sphere1)
  (params (OverlappedComponent :type Primitive%20Component%20Object%20Reference) (OtherActor :type Actor%20Object%20Reference) (OtherComp :type Primitive%20Component%20Object%20Reference) (OtherBodyIndex :type Integer) (bFromSweep :type Boolean) (SweepResult :type Hit%20Result%20Structure%20%28by%20ref%29))
  (if (not (or (== OtherActor self) (== OtherActor "BP_EnemyAI")))
    (Utilities|Casting|CastToBP_SpaceshipCharacter OtherActor)
    ;[1 1 1] Level To Open
    (Game|OpenLevel(byName) (Variables|Default|GetLevelToOpenIfOverlap))))

(event EventTick
  (params (DeltaSeconds :type Float%20%28single-precision%29))
  (bind _charactermovement (Variables|Character|GetCharacterMovement))
  (bind _charactermovement_2 (Variables|Character|GetCharacterMovement))
  (|CallParentFunction DeltaSeconds)
  (Utilities|FlowControl|Sequence
    (:then_0
      (if (Variables|Default|GetPlayerDetected)
        (AI|AIMoveTo self (Math|Vector|MakeVector 0.0 0.0 (.z (Transformation|GetActorLocation))) (Variables|Default|GetCharRef) 1.0 false :!label _label
          (:then
            (Utilities|FlowControl|DoOnce false :!label _label_2
              (:Completed
                (if (Math|Random|RandomBool)
                  (Utilities|FlowControl|Delay (Math|Random|RandomFloatinRange 3.0 6.0))
                  (Components|Activation|Activate (Variables|Default|GetBust1) false)
                  (Variables|/Script/Engine.CharacterMovementComponent|SetMaxWalkSpeed _charactermovement_2 (+ (Variables|/Script/Engine.CharacterMovementComponent|GetMaxWalkSpeed _charactermovement_2) 5e+02))
                  (Utilities|FlowControl|Delay (Math|Random|RandomFloatinRange 1.0 2.0))
                  (Variables|/Script/Engine.CharacterMovementComponent|SetMaxWalkSpeed _charactermovement (- (Variables|/Script/Engine.CharacterMovementComponent|GetMaxWalkSpeed _charactermovement) 5e+02))
                  (goto _label_2 Reset)
                  (else
                    (goto _label_2 Reset))))))
          (:OnSuccess
            (if (not (Variables|Default|GetTakePlayer))
              (goto _label))))
        (else
          (AI|AIMoveTo self (Math|Vector|MakeVector 0.0 0.0 (.z (Transformation|GetActorLocation))) (Variables|Default|GetRoad%20Point%20Ref) 5.0 false))))))

(event EventBeginPlay
  (bind _returnvalue (Actor|GetActorOfClass "/Game/SpaceWalking/Pawns/SpaceshipCharapter/BP_SpaceshipCharacter.BP_SpaceshipCharacter_C"))
  (Variables|Default|SetCharRef _returnvalue))

(fn ConstructionScript
  (|CallParentFunction))