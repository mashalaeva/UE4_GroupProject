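; Game mode for the space-walking level that drives a free camera relative to the spaceship character.
; BeginPlay finds both actors and makes the camera the player's view target.
; AttachCameraToCharacter toggles follow: a timeline glides the camera in X and Y to a fixed offset from the character, then Tick repositions it there each frame, keeping its height.
; DetachCameraFromCharacter is empty, and the actor attach/detach nodes are unconnected.
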(event Custom|AttachCameraToCharacter
  (bind _charref (Variables|Default|GetCharRef))
  (bind _returnvalue (Transformation|GetActorLocation _charref))
  ;[1 1 1] CameraMovement
  (if (Variables|Default|GetCameraAttached)
    (Variables|Default|SetCameraAttached false)
    (elif (not (Variables|Default|GetCameraGoing?))
      (Variables|Default|SetCameraGoing? true)
      (Variables|Default|SetCameraFirstLocation (Transformation|GetActorLocation (Variables|Default|GetCameraRef)))
      (Variables|Default|SetCameraSecondLocation (Math|Vector|MakeVector (- (.x _returnvalue) 2e+03) (.y _returnvalue) (.z _returnvalue)))
      (bind _newtrack_0 (Timeline|Timeline_0 PlayFromStart)
        (:Update
          (Transformation|SetActorLocation (Variables|Default|GetCameraRef) (Math|Vector|Lerp(Vector) (Math|Vector|MakeVector (.x (Variables|Default|GetCameraFirstLocation)) (.y (Variables|Default|GetCameraFirstLocation)) (.z (Variables|Default|GetCameraFirstLocation))) (Math|Vector|MakeVector (.x (Variables|Default|GetCameraSecondLocation)) (.y (Variables|Default|GetCameraSecondLocation)) (.z (Variables|Default|GetCameraFirstLocation))) _newtrack_0) false false))
        (:Finished
          (Variables|Default|SetCameraGoing? false)
          (Variables|Default|SetCameraAttached true))))))

(event Custom|DetachCameraFromCharacter
  ;[1 1 1] Camera Attach/Detach
)

(event Custom|CameraMoveToCharacter
  (bind _charref (Variables|Default|GetCharRef))
  (bind _returnvalue (Transformation|GetActorLocation _charref))
  ;[1 1 1] CameraMovement
  (Transformation|SetActorLocation (Variables|Default|GetCameraRef) (Math|Vector|MakeVector (- (.x _returnvalue) 2e+03) (.y _returnvalue) (.z (Transformation|GetActorLocation (Variables|Default|GetCameraRef)))) false false))

(event EventBeginPlay
  (bind _returnvalue (Actor|GetActorOfClass "/Game/SpaceWalking/Pawns/SpaceshipCharapter/BP_SpaceshipCharacter.BP_SpaceshipCharacter_C"))
  (Variables|Default|SetCharRef _returnvalue)
  (bind _returnvalue_2 (Actor|GetActorOfClass "/Game/SpaceWalking/BP_FreeCamera.BP_FreeCamera_C"))
  (bind _output_get (Variables|Default|SetCameraRef _returnvalue_2))
  (Game|Player|SetViewTargetwithBlend (Game|GetPlayerController 0) _output_get 0.0 "VTBlend_Linear" 0.0 false))

(event EventTick
  (params (DeltaSeconds :type Float%20%28single-precision%29))
  (if (Variables|Default|GetCameraAttached)
    (CallFunction|CameraMovetoCharacter)))

(fn ConstructionScript)