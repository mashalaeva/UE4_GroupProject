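; Game mode for the surface-walking game that provides pause and resume events.
; PauseGame casts the first player controller to BP_SurfaceWalkingPlayerController, shows the mouse cursor, enables its click and mouse-over events, then pauses the game.
; ResumeGame reverses those settings and unpauses.
; If the cast fails, neither event changes the pause state.
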(event Custom|ResumeGame
  (bind _asbp_surface_walking_player_controller (Utilities|Casting|CastToBP_SurfaceWalkingPlayerController (Game|GetPlayerController 0)))
  (Variables|/Script/Engine.PlayerController|SetbShowMouseCursor _asbp_surface_walking_player_controller false)
  (Variables|/Script/Engine.PlayerController|SetbEnableMouseOverEvents _asbp_surface_walking_player_controller false)
  (Variables|/Script/Engine.PlayerController|SetbEnableClickEvents _asbp_surface_walking_player_controller false)
  (Game|SetGamePaused false))

(event Custom|PauseGame
  (bind _asbp_surface_walking_player_controller (Utilities|Casting|CastToBP_SurfaceWalkingPlayerController (Game|GetPlayerController 0)))
  (Variables|/Script/Engine.PlayerController|SetbShowMouseCursor _asbp_surface_walking_player_controller true)
  (Variables|/Script/Engine.PlayerController|SetbEnableMouseOverEvents _asbp_surface_walking_player_controller true)
  (Variables|/Script/Engine.PlayerController|SetbEnableClickEvents _asbp_surface_walking_player_controller true)
  (Game|SetGamePaused true))

(fn ConstructionScript)