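; BP_Chest is an interactable chest actor that shows a text prompt while the player character is near it.
; Its Box overlap events react only to player character 0, toggling the TextRender through ChangeTextVisibility, which also stores the state in IsTextVisible.
; On entry it registers itself as Chest on the SurfaceWalking player controller; leaving hides the text but keeps that reference.
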(event OnComponentBeginOverlap(Box)
  (params (OverlappedComponent :type Primitive%20Component%20Object%20Reference) (OtherActor :type Actor%20Object%20Reference) (OtherComp :type Primitive%20Component%20Object%20Reference) (OtherBodyIndex :type Integer) (bFromSweep :type Boolean) (SweepResult :type Hit%20Result%20Structure%20%28by%20ref%29))
  (bind _asbp_surface_walking_character (Utilities|Casting|CastToBP_SurfaceWalkingCharacter OtherActor))
  (bind _asbp_surface_walking_character_2 (Utilities|Casting|CastToBP_SurfaceWalkingCharacter (Game|GetPlayerCharacter 0)))
  (if (== _asbp_surface_walking_character_2 _asbp_surface_walking_character)
    (bind _asbp_surface_walking_player_controller (Utilities|Casting|CastToBP_SurfaceWalkingPlayerController (Game|GetPlayerController 0)))
    (Variables|/Game/SurfaceWalking/Pawns/Character/BP_SurfaceWalkingPlayerController.BP_SurfaceWalkingPlayerController_C|SetChest _asbp_surface_walking_player_controller self)
    (CallFunction|ChangeTextVisibility true)))

(event OnComponentEndOverlap(Box)
  (params (OverlappedComponent :type Primitive%20Component%20Object%20Reference) (OtherActor :type Actor%20Object%20Reference) (OtherComp :type Primitive%20Component%20Object%20Reference) (OtherBodyIndex :type Integer))
  (bind _asbp_surface_walking_character (Utilities|Casting|CastToBP_SurfaceWalkingCharacter OtherActor))
  (bind _asbp_surface_walking_character_2 (Utilities|Casting|CastToBP_SurfaceWalkingCharacter (Game|GetPlayerCharacter 0)))
  (if (== _asbp_surface_walking_character_2 _asbp_surface_walking_character)
    (CallFunction|ChangeTextVisibility false)))

(event Custom|ChangeTextVisibility
  (params (IsVisible? :type Boolean))
  (Rendering|SetVisibility (Variables|Default|GetTextRender) IsVisible? false)
  (Variables|Default|SetIsTextVisible? IsVisible?))

(fn ConstructionScript)