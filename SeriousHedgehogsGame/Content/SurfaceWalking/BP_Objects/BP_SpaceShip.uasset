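; BP_SpaceShip is the surface-walking level's exit point that sends the player to the Space level.
; When the player's surface-walking character overlaps its collision box, it copies the player controller's inventory component contents into BP_GameInstance so they persist across the level change.
; It then stores "Space" as the level to load on the game instance and opens that level by name.
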(event OnComponentBeginOverlap(CollisionBox)
  (params (OverlappedComponent :type Primitive%20Component%20Object%20Reference) (OtherActor :type Actor%20Object%20Reference) (OtherComp :type Primitive%20Component%20Object%20Reference) (OtherBodyIndex :type Integer) (bFromSweep :type Boolean) (SweepResult :type Hit%20Result%20Structure%20%28by%20ref%29))
  (bind _asbp_surface_walking_character (Utilities|Casting|CastToBP_SurfaceWalkingCharacter (Game|GetPlayerCharacter 0)))
  (if (== _asbp_surface_walking_character OtherActor)
    (bind _asbp_surface_walking_player_controller (Utilities|Casting|CastToBP_SurfaceWalkingPlayerController (Game|GetPlayerController 0)))
    (bind _asbp_game_instance (Utilities|Casting|CastToBP_GameInstance (Game|GetGameInstance)))
    (Variables|/Game/General/BP_GameInstance.BP_GameInstance_C|SetInventory _asbp_game_instance (Variables|/Game/SurfaceWalking/Inventory/InventoryComponent.InventoryComponent_C|GetInventory (Variables|/Game/SurfaceWalking/Pawns/Character/BP_SurfaceWalkingPlayerController.BP_SurfaceWalkingPlayerController_C|GetInventoryComponent _asbp_surface_walking_player_controller)))
    (bind _output_get (Variables|/Game/General/BP_GameInstance.BP_GameInstance_C|SetLevelToLoad _asbp_game_instance "Space"))
    (Game|OpenLevel(byName) _output_get)))

(event EventBeginPlay)

(event Collision|EventActorBeginOverlap
  (params (OtherActor :type Actor%20Object%20Reference)))

(event EventTick
  (params (DeltaSeconds :type Float%20%28single-precision%29)))

(fn ConstructionScript)