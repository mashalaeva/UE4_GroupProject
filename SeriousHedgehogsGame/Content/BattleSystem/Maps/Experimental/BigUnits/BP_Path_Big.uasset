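; BP_Path_Big is a pathfinding variant that finds reachable tiles for multi-tile units on the battle grid.
; RunPathfinding reads the size of the BP_Unit_Big on the start tile, defaulting to 1, then runs the parent search.
; AddTileIfValid admits tiles within move range whose GridBigIndexes value fits that size.
; Tiles held by other units are recorded as reachable units but not expanded, while the moving unit's own tiles stay open.
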(fn AddTileifValid
  (params (EdgeIndex :type Integer%20%28by%20ref%29) (TotalCost :type Integer%20%28by%20ref%29) (ParentIndex :type Integer%20%28by%20ref%29) (Move :type Integer%20%28by%20ref%29) (Paths :type Map%20of%20Integers%20to%20Structs) (OpenListChildTiles :type Array%20of%20F%20Pathfinding%20Index%20Structures))
  (bind _gridmanagerref (Variables|Default|GetGridManagerRef))
  (bind _gridunits (Variables|/Game/BattleSystem/Core/Grid/BP_GridManager.BP_GridManager_C|GetGridUnits _gridmanagerref))
  (bind (_value _returnvalue) (Utilities|Map|Find _gridunits EdgeIndex))
  (if (>= (.Value (Utilities|Map|Find (Variables|/Game/BattleSystem/Core/Grid/BP_GridManager.BP_GridManager_C|GetGridBigIndexes (Variables|Default|GetGridManagerRef)) EdgeIndex)) (Variables|Default|GetUnitSize))
    (if (<= TotalCost Move)
      (Utilities|Map|Add Paths EdgeIndex (Utilities|Struct|MakeFPathfinding TotalCost ParentIndex))
      (if _returnvalue
        (if (!= _value (Variables|Default|GetTriggeringUnit))
          (Utilities|Set|Add (Variables|Default|GetReachableUnitIndexes) EdgeIndex)
          (else
            (Utilities|Array|Add OpenListChildTiles (Utilities|Struct|MakeFPathfindingIndex EdgeIndex TotalCost ParentIndex) :!label _label)))
        (else
          (goto _label)))
      (return))
    (else
      (return))))

(fn RunPathfinding
  (params (StartIndex :type Integer) (MoveRange :type Integer) (GridManager :type BP%20Grid%20Manager%20Object%20Reference))
  (bind _asbp_unit_big (Utilities|Casting|CastToBP_Unit_Big (.Value (Utilities|Map|Find (Variables|/Game/BattleSystem/Core/Grid/BP_GridManager.BP_GridManager_C|GetGridUnits GridManager) StartIndex)))
    (:then
      (bind _output_get (Variables|Default|SetTriggeringUnit _asbp_unit_big))
      (Variables|Default|SetUnitSize (Variables|/Game/BattleSystem/Maps/Experimental/BigUnits/BP_Unit_Big.BP_Unit_Big_C|GetSize _output_get)))
    (:CastFailed
      (Variables|Default|SetUnitSize 1)))
  (bind (_pathsmap _pathobject) (|CallParentFunction StartIndex MoveRange GridManager))
  (return _pathsmap _pathobject))