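; Laser rifle ability for grid-based tactical battles that deals random ranged damage to a unit.
; Hit chance combines accuracy, dodge and BP_CoverSystem cover and distance; ShootUnit applies damage and queues BP_Action_LaserRifle, with attack cam on some shots.
; Execution wakes units near shooter and target, but active AI units with DemoOverwatch may choose overwatch when odds are poor.
; AI targeting favors close, killable units and weights tiles by hit chance.
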(fn ConstructionScript
  (|CallParentFunction))

(fn GetDescription
  (bind _damagerange (Variables|Default|GetDamageRange))
  (return "Laser Rifle" (Utilities|Text|ToText(String) (Utilities|String|Append (Utilities|String|ToString(Text) (Utilities|Text|MakeLiteralText "Fire a laser beam for ")) "" (Utilities|String|ToString(Integer) (.min _damagerange)) " - " (Utilities|String|ToString(Integer) (.max _damagerange)) (Utilities|String|ToString(Text) (Utilities|Text|MakeLiteralText " points of damage at 
an enemy. Accuracy decreases with distance."))))))

(fn GetHoverText
  (params (HoveredTile :type Integer))
  (bind _gridmanagerref (Variables|Default|GetGridManagerRef))
  (bind _owningunit (Variables|Default|GetOwningUnit))
  (bind _damagerange (Variables|Default|GetDamageRange))
  (bind _damagerange_2 (Variables|Default|GetDamageRange))
  (bind _gridunits (Variables|/Game/BattleSystem/Core/Grid/BP_GridManager.BP_GridManager_C|GetGridUnits _gridmanagerref))
  (bind (_value _returnvalue) (Utilities|Map|Find _gridunits HoveredTile))
  (if _returnvalue
    (if (Utilities|Set|Contains (Variables|/Game/BattleSystem/Core/Units/BP_Unit.BP_Unit_C|GetAlliedFactions (Variables|Default|GetOwningUnit)) (Variables|/Game/BattleSystem/Core/Units/BP_Unit.BP_Unit_C|GetFaction _value))
      (return "Laser Rifle" (Utilities|Text|ToText(String) (Utilities|String|Append "Hit Chance: " "-" " 
Damage: " (Utilities|String|ToString(Integer) (.min _damagerange)) " - " (Utilities|String|ToString(Integer) (.max _damagerange)))))
      (elif (<= (Default|FindDistanceIinTilesBetweenIndexes (Variables|Default|GetGridManagerRef) HoveredTile (Variables|/Game/BattleSystem/Core/Units/BP_Unit.BP_Unit_C|GetGridIndex _owningunit) (Variables|/Game/BattleSystem/Core/Units/BP_Unit.BP_Unit_C|GetbDiamondShapedVisibility _owningunit)) (Variables|Default|GetRange))
        (bind _bvisible (Default|CheckifTileIsVisiblefromOtherTile (Variables|Default|GetGridManagerRef) (Variables|/Game/BattleSystem/Core/Units/BP_Unit.BP_Unit_C|GetGridIndex (Variables|Default|GetOwningUnit)) HoveredTile (* (Variables|Default|GetRange) (Variables|/Game/BattleSystem/Core/Grid/BP_GridManager.BP_GridManager_C|GetTileXSize (Variables|Default|GetGridManagerRef))) 1 true false))
        (if _bvisible
          (bind _hit_chance (CallFunction|FindHitChanceandifHit (Variables|Default|GetOwningUnit) HoveredTile))
          (return "Laser Rifle" (Utilities|Text|ToText(String) (Utilities|String|Append "Hit Chance: " (Utilities|String|ToString(Integer) (Math|Float|Floor (* _hit_chance 1e+02))) "% 
Damage: " (Utilities|String|ToString(Integer) (.min _damagerange_2)) " - " (Utilities|String|ToString(Integer) (.max _damagerange_2))))))))
    (else
      (return "Laser Rifle" (Utilities|Text|ToText(String) (Utilities|String|Append "Hit Chance: " "-" " 
Damage: " (Utilities|String|ToString(Integer) (.min _damagerange)) " - " (Utilities|String|ToString(Integer) (.max _damagerange))))))))

(fn FindHitChanceandifHit
  (params (ShootingUnit :type BP%20Unit%20Object%20Reference) (TargetIndex :type Integer))
  (bind _gridmanagerref (Variables|Default|GetGridManagerRef))
  (bind _gridmanagerref_2 (Variables|Default|GetGridManagerRef))
  (bind _returnvalue (Actor|GetComponentbyClass _gridmanagerref_2 "/Game/BattleSystem/Core/Grid/BP_CoverSystem.BP_CoverSystem_C"))
  (bind _returnvalue_2 (Actor|GetComponentbyClass ShootingUnit "/Game/BattleSystem/Core/Units/BP_ExtraAttributes.BP_ExtraAttributes_C"))
  (bind _gridunits (Variables|/Game/BattleSystem/Core/Grid/BP_GridManager.BP_GridManager_C|GetGridUnits _gridmanagerref))
  (bind _value (Utilities|Map|Find _gridunits TargetIndex))
  (bind _returnvalue_3 (Actor|GetComponentbyClass _value "/Game/BattleSystem/Core/Units/BP_ExtraAttributes.BP_ExtraAttributes_C"))
  (if (Utilities|IsValid _returnvalue)
    (bind (_hit _hit_chance) (Default|CalculateHitChance _returnvalue (- (Math|Float|SelectFloat (Variables|/Game/BattleSystem/Core/Units/BP_ExtraAttributes.BP_ExtraAttributes_C|GetAccuracy _returnvalue_2) 1.0 (Utilities|IsValid _returnvalue_2)) (Math|Float|SelectFloat (Variables|/Game/BattleSystem/Core/Units/BP_ExtraAttributes.BP_ExtraAttributes_C|GetDodge _returnvalue_3) 0.0 (Utilities|IsValid _returnvalue_3))) 0.05 0.0 (Variables|/Game/BattleSystem/Core/Units/BP_Unit.BP_Unit_C|GetGridIndex ShootingUnit) TargetIndex (Variables|/Game/BattleSystem/Core/Units/BP_Unit.BP_Unit_C|GetbDiamondShapedVisibility ShootingUnit)))
    (return _hit _hit_chance)
    (else
      (return true 1.0))))

(fn FindTargetValue
  (params (TargetIndex :type Integer))
  (bind _gridmanagerref (Variables|Default|GetGridManagerRef))
  (bind _gridunits (Variables|/Game/BattleSystem/Core/Grid/BP_GridManager.BP_GridManager_C|GetGridUnits _gridmanagerref))
  (bind _value (Utilities|Map|Find _gridunits TargetIndex))
  (bind _currenthealth (Variables|/Game/BattleSystem/Core/Units/BP_Unit.BP_Unit_C|GetCurrentHealth _value))
  (return (* (/ 1.0 (Math|Conversions|ToFloat(Integer) (+ (Default|FindDistanceIinTilesBetweenIndexes (Variables|Default|GetGridManagerRef) TargetIndex (Variables|/Game/BattleSystem/Core/Units/BP_Unit.BP_Unit_C|GetGridIndex (Variables|Default|GetOwningUnit)) false) 9))) (Utilities|Select :Index (+ (Math|Conversions|ToInteger(Boolean) (<= (- (Math|Float|Truncate _currenthealth) (.min (Variables|Default|GetDamageRange))) 0)) (Math|Conversions|ToInteger(Boolean) (<= (- (Math|Float|Truncate _currenthealth) (.max (Variables|Default|GetDamageRange))) 0))) :Option%200 3.0 :Option%201 5.0 :Option%202 1e+01))))

(fn RenderBeam
  (params (OwningUnit :type Actor%20Object%20Reference) (TargetLocation :type Vector))
  (bind _returnvalue (Actor|GetComponentsbyTag OwningUnit "/Script/Engine.StaticMeshComponent" "Weapon"))
  (bind _output (Utilities|Array|Get(acopy) _returnvalue))
  (bind _returnvalue_2 (Transformation|GetSocketLocation _output "Muzzle"))
  (if (not (Networking|IsDedicatedServer))
    (if (Utilities|IsValid _output)
      (Audio|PlaySoundatLocation "/Game/BattleSystem/Maps/Advanced/Abilities/A_Laser.A_Laser" _returnvalue_2 "0, 0, 0" 1.0 1.0 0.0 0 0 0)
      (bind _returnvalue_3 (Effects|SpawnEmitterAttached "/Game/BattleSystem/Maps/Advanced/Abilities/PS_Laser.PS_Laser" _output "Muzzle" _returnvalue_2))
      (Class|ParticleSystemComponent|SetBeamSourcePoint _returnvalue_3 0 _returnvalue_2)
      (Class|ParticleSystemComponent|SetBeamTargetPoint _returnvalue_3 0 TargetLocation)
      (Rendering|SetVisibility _returnvalue_3 true false)
      (return)
      (else
        (return)))))

(fn ShootUnit
  (params (ShootingUnit :type BP%20Unit%20Object%20Reference) (TargetUnitIn :type BP%20Unit%20Object%20Reference) (bAutoAnimate :type Boolean))
  (bind _gridmanager (CallFunction|GetGridManager))
  (bind _damagerange (Variables|Default|GetDamageRange))
  (bind _hit (CallFunction|FindHitChanceandifHit ShootingUnit (Variables|/Game/BattleSystem/Core/Units/BP_Unit.BP_Unit_C|GetGridIndex TargetUnitIn)))
  (LocalVariables|SetbLocalHit _hit)
  (Utilities|FlowControl|Sequence
    (:then_0
      (LocalVariables|SetDamageStored (Math|Conversions|ToFloat(Integer) (Math|Random|RandomIntegerinRange (.min _damagerange) (.max _damagerange))))
      (if bAutoAnimate
        (bind _output_get (LocalVariables|SetbLocalUseAttackCam (or (and (<= (- (Variables|/Game/BattleSystem/Core/Units/BP_Unit.BP_Unit_C|GetCurrentHealth TargetUnitIn) (LocalVariables|GetDamageStored)) 0.0) (LocalVariables|GetbLocalHit)) (!= (Variables|/Game/BattleSystem/Core/BP_TurnManager.BP_TurnManager_C|GetActiveActorAnimate (.TurnManager (CallFunction|GetTurnManager))) (Variables|Default|GetOwningActor)))))
        (if _output_get
          _
          (else
            (Default|QueuePanCamera (.GridCamera (CallFunction|GetGridCamera)) (CallFunction|GetLocationBetweenUnits ShootingUnit TargetUnitIn) 0 0.5)))
        (Game|SpawnActorfromClass "/Game/BattleSystem/Maps/Advanced/Actions/BP_Action_LaserRifle.BP_Action_LaserRifle_C" (Math|Transform|MakeTransform "0, 0, 0" "0, 0, 0" "1,1,1") "Undefined" 0 (Variables|/Game/BattleSystem/Core/Units/BP_Unit.BP_Unit_C|GetPuppet ShootingUnit) (LocalVariables|GetbLocalHit) (Default|ConvertfromGridtoWorld _gridmanager (+ (.Value (Utilities|Map|Find (Variables|/Game/BattleSystem/Core/Grid/BP_GridManager.BP_GridManager_C|GetGridLocations _gridmanager) (Variables|/Game/BattleSystem/Core/Units/BP_Unit.BP_Unit_C|GetGridIndex TargetUnitIn))) "0, 0,100.000000")) (Variables|/Game/BattleSystem/Core/Units/BP_Unit.BP_Unit_C|GetPuppet TargetUnitIn) (LocalVariables|GetDamageStored) (<= (- (Variables|/Game/BattleSystem/Core/Units/BP_Unit.BP_Unit_C|GetCurrentHealth TargetUnitIn) (LocalVariables|GetDamageStored)) 0.0) (LocalVariables|GetbLocalUseAttackCam) (!= (Variables|/Game/BattleSystem/Core/BP_TurnManager.BP_TurnManager_C|GetActiveActorAnimate (.TurnManager (CallFunction|GetTurnManager))) (Variables|Default|GetOwningActor)) (Math|Float|SelectFloat -1.0 1.0 (LocalVariables|GetbLocalHit)) "NewEnumerator0" 0)))
    (:then_1
      (if (LocalVariables|GetbLocalHit)
        (Default|ModifyHealth TargetUnitIn (* (LocalVariables|GetDamageStored) -1.0) false 1.0))
      (return (LocalVariables|GetbLocalHit) TargetUnitIn (LocalVariables|GetDamageStored)))))

(fn FindAbilitySpecificTileValueModifier
  (params (GridIndex :type Integer) (TargetIndex :type Integer))
  (bind _hit_chance (Default|CalculateHitChance (Actor|GetComponentbyClass (Variables|Default|GetGridManagerRef) "/Game/BattleSystem/Core/Grid/BP_CoverSystem.BP_CoverSystem_C") 1.0 0.05 0.0 TargetIndex GridIndex false))
  (return _hit_chance))

(fn ExecuteAbility
  (params (TargetIndexIn :type Integer))
  (bind _busedoverwatch (CallFunction|ActivateAiOverwatchifOptimal TargetIndexIn))
  (if _busedoverwatch
    (return true)
    (else
      (CallFunction|ShootUnit (Variables|Default|GetOwningUnit) (.Value (Utilities|Map|Find (Variables|/Game/BattleSystem/Core/Grid/BP_GridManager.BP_GridManager_C|GetGridUnits (Variables|Default|GetGridManagerRef)) TargetIndexIn)) true)
      (CallFunction|WakeNearbyUnits TargetIndexIn 6 10)
      (CallFunction|WakeNearbyUnits (Variables|/Game/BattleSystem/Core/Units/BP_Unit.BP_Unit_C|GetGridIndex (Variables|Default|GetOwningUnit)) 10 10)
      (return true))))

(fn ActivateAiOverwatchifOptimal
  (params (TargetIndex :type Integer))
  (bind _gridmanagerref (Variables|Default|GetGridManagerRef))
  (bind _owningunit (Variables|Default|GetOwningUnit))
  (bind _owningunit_2 (Variables|Default|GetOwningUnit))
  (bind _owningunit_3 (Variables|Default|GetOwningUnit))
  (bind _returnvalue (Actor|GetComponentbyClass _owningunit_3 "/Game/BattleSystem/Core/Units/BP_ExtraAttributes.BP_ExtraAttributes_C"))
  (bind _gridunits (Variables|/Game/BattleSystem/Core/Grid/BP_GridManager.BP_GridManager_C|GetGridUnits _gridmanagerref))
  (bind _value (Utilities|Map|Find _gridunits TargetIndex))
  (bind _returnvalue_2 (Actor|GetComponentbyClass _value "/Game/BattleSystem/Core/Units/BP_ExtraAttributes.BP_ExtraAttributes_C"))
  (if (and (Variables|/Game/BattleSystem/Core/Units/BP_Unit.BP_Unit_C|GetbAIControlled _owningunit_2) (Utilities|Array|ContainsItem (Variables|/Game/BattleSystem/Core/Units/BP_AbilitySystem.BP_AbilitySystem_C|GetAbilities (Actor|GetComponentbyClass _owningunit_2 "/Game/BattleSystem/Core/Units/BP_AbilitySystem.BP_AbilitySystem_C")) "/Game/BattleSystem/Maps/Advanced/Abilities/BP_Ability_DemoOverwatch.BP_Ability_DemoOverwatch_C"))
    (if (== (Variables|/Game/BattleSystem/Core/BP_TurnManager.BP_TurnManager_C|GetActiveUnit (.TurnManager (CallFunction|GetTurnManager))) (Variables|Default|GetOwningUnit))
      (bind _hit_chance (Default|CalculateHitChance (Actor|GetComponentbyClass (Variables|Default|GetGridManagerRef) "/Game/BattleSystem/Core/Grid/BP_CoverSystem.BP_CoverSystem_C") (- (Math|Float|SelectFloat (Variables|/Game/BattleSystem/Core/Units/BP_ExtraAttributes.BP_ExtraAttributes_C|GetAccuracy _returnvalue) 1.0 (Utilities|IsValid _returnvalue)) (Math|Float|SelectFloat (Variables|/Game/BattleSystem/Core/Units/BP_ExtraAttributes.BP_ExtraAttributes_C|GetDodge _returnvalue_2) 0.0 (Utilities|IsValid _returnvalue_2))) 0.05 0.0 (Variables|/Game/BattleSystem/Core/Units/BP_Unit.BP_Unit_C|GetGridIndex _owningunit) TargetIndex (Variables|/Game/BattleSystem/Core/Units/BP_Unit.BP_Unit_C|GetbDiamondShapedVisibility _owningunit)))
      (if (< _hit_chance (Math|Random|RandomFloatinRangefromStream 0.0 (Variables|Default|GetAiOverwatchThreshold) (Variables|Default|GetOverwatchStream)))
        (CallFunction|AddStatusEffect "/Game/BattleSystem/Maps/Advanced/Abilities/BP_SE_Overwatch.BP_SE_Overwatch_C" (Variables|Default|GetOwningUnit))
        (return true)
        (else
          (return false)))
      (else
        (return false)))
    (else
      (return false))))