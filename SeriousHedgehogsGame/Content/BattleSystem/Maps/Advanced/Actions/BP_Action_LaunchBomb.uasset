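; Battle action that has the source puppet lob a bomb along an arc to a target location.
; On the puppet's attack animation event, it spawns BP_Bomb at the gun muzzle with a suggested arc velocity.
; Tick detonates it near the target with effect and sound, destroys it and ends the action.
; A delayed failsafe event can force the same explosion, though nothing here calls it.
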(event Custom|ExplodeBombAfterDelayIfExists
  (Utilities|FlowControl|Delay (Variables|Default|GetFailsafeCheckDelay))
  (Utilities|IsValid (Variables|Default|GetBomb)
    (:Is%20Valid
      (Effects|SpawnEmitteratLocation "/Game/BattleSystem/Maps/Advanced/Abilities/PS_Explosion.PS_Explosion" (Variables|Default|GetEnd%20Pos) "0, 0, 0" "5.000000,5.000000,5.000000")
      (Audio|PlaySoundatLocation "/Game/BattleSystem/Maps/2D/Items/A_Fireblast_Hit_Cue.A_Fireblast_Hit_Cue" (Variables|Default|GetEnd%20Pos) "0, 0, 0" 1.0 1.0 0.0 0 0 0)
      (Actor|Tick|SetActorTickEnabled false)
      (Actor|DestroyActor (Variables|Default|GetBomb))
      (CallFunction|EndAction true))))

(event Custom|AttackHit
  (params (AnimatingActor :type Actor%20Object%20Reference) (Animation :type Gameplay%20Tag%20Structure))
  (EventDispatchers|UnbindEventfromOnAnimationEnd (Actor|GetComponentbyClass (Variables|Default|GetSourcePuppet) "/Game/BattleSystem/Core/Units/BP_PuppetComponent.BP_PuppetComponent_C") (delegate Custom|AttackHit))
  (bind _muzzletransform (Class|BPIUnitHUD|GetGunMuzzle(Message) (Variables|Default|GetSourcePuppet)))
  (bind _outlaunchvelocity (Game|SuggestProjectileVelocityCustomArc (.location _muzzletransform) (Variables|Default|GetEnd%20Pos) 0.0 (Variables|Default|GetArc%20Param)))
  (bind _returnvalue (Game|SpawnActorfromClass "/Game/BattleSystem/Maps/Advanced/Abilities/BP_Bomb.BP_Bomb_C" (Math|Transform|MakeTransform (.location _muzzletransform) "0, 0, 0" "0.200000,0.200000,0.200000") "AlwaysSpawn" 0 _outlaunchvelocity 0))
  (Variables|Default|SetBomb _returnvalue)
  (Actor|Tick|SetActorTickEnabled true))

(event EventTick
  (params (DeltaSeconds :type Float%20%28single-precision%29))
  (if (Math|Vector|Equal(Vector) (Variables|Default|GetEnd%20Pos) (Transformation|GetWorldLocation (Variables|/Game/BattleSystem/Maps/Advanced/Abilities/BP_Bomb.BP_Bomb_C|GetStaticMesh (Variables|Default|GetBomb))) 4e+01)
    (Effects|SpawnEmitteratLocation "/Game/BattleSystem/Maps/Advanced/Abilities/PS_Explosion.PS_Explosion" (Variables|Default|GetEnd%20Pos) "0, 0, 0" "5.000000,5.000000,5.000000")
    (Audio|PlaySoundatLocation "/Game/BattleSystem/Maps/2D/Items/A_Fireblast_Hit_Cue.A_Fireblast_Hit_Cue" (Variables|Default|GetEnd%20Pos) "0, 0, 0" 1.0 1.0 0.0 0 0 0)
    (Actor|Tick|SetActorTickEnabled false)
    (Actor|DestroyActor (Variables|Default|GetBomb))
    (CallFunction|EndAction true)))

(event EventPlayAction
  (EventDispatchers|BindEventtoOnAnimationEvent (Actor|GetComponentbyClass (Variables|Default|GetSourcePuppet) "/Game/BattleSystem/Core/Units/BP_PuppetComponent.BP_PuppetComponent_C") (delegate Custom|AttackHit))
  (Class|BPIPuppet|AnimatePuppet(Message) (Variables|Default|GetSourcePuppet) "(TagName=\"Anim.Attack\")" (Variables|Default|GetEnd%20Pos)))

(fn ConstructionScript
  (|CallParentFunction))