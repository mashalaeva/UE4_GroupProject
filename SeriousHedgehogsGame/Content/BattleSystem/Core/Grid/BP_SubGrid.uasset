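; BP_SubGrid is a placeable secondary grid in the battle system that aligns itself to the level's BP_GridManager.
; Its construction script snaps the anchor to the closest manager tile and stores the relative grid index.
; It optionally sizes heightmap bounds from manager settings and fills the subgrid with instanced tile meshes.
; PreventSubgridOverlap, uncalled here, moves the actor out to the main grid's far edge or snaps it to grid coordinates.
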(event EventBeginPlay)

(event Collision|EventActorBeginOverlap
  (params (OtherActor :type Actor%20Object%20Reference)))

(event EventTick
  (params (DeltaSeconds :type Float%20%28single-precision%29)))

(fn ConstructionScript
  (bind _tilemeshoverride (Variables|Default|GetTileMeshOverride))
  (bind _outactors (Actor|GetAllActorsOfClass "/Game/BattleSystem/Core/Grid/BP_GridManager.BP_GridManager_C"))
  (if (> (Utilities|Array|Length _outactors) 0)
    (Variables|Default|SetGridManagerRef (Utilities|Array|Get(acopy) _outactors))
    (bind _snaplocation (Default|FindClosestTiletoSnapto (Variables|Default|GetGridManagerRef) (Transformation|GetActorLocation)))
    (Transformation|SetWorldLocation (Variables|Default|GetBP_GridAnchor) (Math|Vector|MakeVector (.x _snaplocation) (.y _snaplocation) (.z (Transformation|GetActorLocation (Variables|Default|GetGridManagerRef)))) false false)
    (Variables|Default|SetRelativeGridIndex (.Index (Default|ConvertLocationtoIndex3D (Variables|Default|GetGridManagerRef) (Transformation|GetActorLocation))))
    (Rendering|SetVisibility (Variables|Default|GetHeightmapBounds) (Variables|Default|GetbShowBounds) false)
    (if (Variables|Default|GetbShowBounds)
      (CallFunction|AdjustHeightmapBounds))
    (if (Variables|Default|GetbSpawnGridMeshes)
      (Components|StaticMesh|SetStaticMesh (Variables|Default|GetDefaultTile) (select (Utilities|IsValid _tilemeshoverride) _tilemeshoverride (Variables|/Game/BattleSystem/Core/Grid/BP_GridManager.BP_GridManager_C|GetDefaultTileMesh (Variables|Default|GetGridManagerRef))))
      (CallFunction|SpawnGridMeshes)
      (Development|SetHiddeninGame (Variables|Default|GetDefaultTile) false false)
      (else
        (Development|SetHiddeninGame (Variables|Default|GetDefaultTile) true false)))))

(fn PreventSubgridOverlap
  (bind _returnvalue (Transformation|GetActorLocation))
  (bind _gridmanagerref (Variables|Default|GetGridManagerRef))
  (bind _gridmanagerref_2 (Variables|Default|GetGridManagerRef))
  (bind _gridmanagerref_3 (Variables|Default|GetGridManagerRef))
  (bind _gridmanagerref_4 (Variables|Default|GetGridManagerRef))
  (bind ___ (Default|ConvertfromWorldtoGrid _gridmanagerref _returnvalue))
  (bind _tilexsize (Variables|/Game/BattleSystem/Core/Grid/BP_GridManager.BP_GridManager_C|GetTileXSize _gridmanagerref_4))
  (bind _gridsizex (Variables|/Game/BattleSystem/Core/Grid/BP_GridManager.BP_GridManager_C|GetGridSizeX _gridmanagerref_2))
  (bind _gridsizey (Variables|/Game/BattleSystem/Core/Grid/BP_GridManager.BP_GridManager_C|GetGridSizeY _gridmanagerref_2))
  (bind _tilexsize_2 (Variables|/Game/BattleSystem/Core/Grid/BP_GridManager.BP_GridManager_C|GetTileXSize _gridmanagerref_2))
  (bind _returnvalue_2 (* _gridsizex _tilexsize_2))
  (bind _returnvalue_3 (* _gridsizey _tilexsize_2))
  (bind _returnvalue_4 (Math|Float|Max(Float) (.x ___) 0.0))
  (bind _returnvalue_5 (Math|Float|Max(Float) (.y ___) 0.0))
  (bind ____2 (Default|ConvertfromGridtoWorld _gridmanagerref_3 (Math|Vector|MakeVector _returnvalue_4 _returnvalue_5 (.z ___))))
  (bind (_x _y) (Math|Vector|BreakVector ____2))
  (bind (_x_2 _y_2 _z) (Math|Vector|BreakVector ____2))
  (bind _returnvalue_6 (- _y _returnvalue_3))
  (bind _returnvalue_7 (- _x _returnvalue_2))
  (bind _returnvalue_8 (Math|Float|Absolute(Float) _returnvalue_6))
  (bind _returnvalue_9 (Math|Float|Absolute(Float) _returnvalue_7))
  (bind _returnvalue_10 (> _returnvalue_9 _returnvalue_8))
  (if (and (< _x _returnvalue_2) (< _y _returnvalue_3))
    (Transformation|SetActorLocation (Math|Vector|MakeVector (Math|Float|SelectFloat _x_2 (* (Variables|/Game/BattleSystem/Core/Grid/BP_GridManager.BP_GridManager_C|GetGridSizeX _gridmanagerref_4) _tilexsize) _returnvalue_10) (Math|Float|SelectFloat (* (Variables|/Game/BattleSystem/Core/Grid/BP_GridManager.BP_GridManager_C|GetGridSizeY _gridmanagerref_4) _tilexsize) _y_2 _returnvalue_10) _z) false false)
    (return)
    (else
      (Transformation|SetActorLocation ____2 false false)
      (return))))

(fn SpawnGridMeshes
  (bind _bp_gridanchor (Variables|Default|GetBP_GridAnchor))
  (bind _relativelocation (Variables|/Script/Engine.SceneComponent|GetRelativeLocation _bp_gridanchor))
  (Transformation|SetRelativeLocation (Variables|Default|GetDefaultTile) (Math|Vector|MakeVector (.x _relativelocation) (.y _relativelocation) (Utilities|Select :Index (Variables|/Game/BattleSystem/Core/Grid/BP_GridManager.BP_GridManager_C|GetHeightmap (Variables|Default|GetGridManagerRef)) :NewEnumerator0 (.z _relativelocation) :NewEnumerator2 0.0 :NewEnumerator3 0.0)) false false)
  (for _index (range 0 (- (* (Variables|Default|GetGridSizeX) (Variables|Default|GetGridSizeY)) 1))
    (Components|InstancedStaticMesh|AddInstance (Variables|Default|GetDefaultTile) (Math|Transform|MakeTransform (Default|GetDisplayTileLocationfromIndex (Variables|Default|GetGridManagerRef) _index (Variables|Default|GetGridSizeX) (Variables|Default|GetGridSizeY)) "0, 0, 0" "1,1,1")))
  (return))

(fn AdjustHeightmapBounds
  (bind _gridmanagerref (Variables|Default|GetGridManagerRef))
  (bind _gridmanagerref_2 (Variables|Default|GetGridManagerRef))
  (bind _gridmanagerref_3 (Variables|Default|GetGridManagerRef))
  (bind _gridmanagerref_4 (Variables|Default|GetGridManagerRef))
  (bind _gridsizex (Variables|Default|GetGridSizeX))
  (bind _gridsizey (Variables|Default|GetGridSizeY))
  (bind (_location _scalex _scaley) (Default|SetCollisionPlaneandHeightmapBoxScaleandLocation _gridmanagerref_2 true _gridsizex _gridsizey))
  (bind _maxgridheight (Variables|/Game/BattleSystem/Core/Grid/BP_GridManager.BP_GridManager_C|GetMaxGridHeight _gridmanagerref_3))
  (bind _mingridheight (Variables|/Game/BattleSystem/Core/Grid/BP_GridManager.BP_GridManager_C|GetMinGridHeight _gridmanagerref_3))
  (bind _defaulttilewidth (Variables|/Game/BattleSystem/Core/Grid/BP_GridManager.BP_GridManager_C|GetDefaultTileWidth _gridmanagerref))
  (bind _heightmap (Variables|/Game/BattleSystem/Core/Grid/BP_GridManager.BP_GridManager_C|GetHeightmap _gridmanagerref))
  (bind _maxgridheight_2 (Variables|/Game/BattleSystem/Core/Grid/BP_GridManager.BP_GridManager_C|GetMaxGridHeight _gridmanagerref_4))
  (bind _mingridheight_2 (Variables|/Game/BattleSystem/Core/Grid/BP_GridManager.BP_GridManager_C|GetMinGridHeight _gridmanagerref_4))
  (bind _returnvalue (- _maxgridheight _mingridheight))
  (bind (_x _y) (Math|Vector|BreakVector _location))
  (bind _returnvalue_2 (+ _maxgridheight_2 _mingridheight_2))
  (bind _returnvalue_3 (/ _returnvalue _defaulttilewidth))
  (bind _returnvalue_4 (/ _returnvalue_2 2.0))
  (Transformation|SetRelativeTransform (Variables|Default|GetHeightmapBounds) (Math|Transform|MakeTransform (Math|Vector|MakeVector _x _y (Utilities|Select :Index _heightmap :NewEnumerator0 0.0 :NewEnumerator2 _returnvalue_4 :NewEnumerator3 _returnvalue_4)) "0, 0, 0" (Math|Vector|MakeVector _scalex _scaley (Utilities|Select :Index _heightmap :NewEnumerator0 0.0 :NewEnumerator2 _returnvalue_3 :NewEnumerator3 _returnvalue_3))) false false)
  (return))