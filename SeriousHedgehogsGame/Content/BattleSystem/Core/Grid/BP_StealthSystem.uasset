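; BP_StealthSystem is a stealth component for BP_GridManager that drives noise and sight detection on the battle grid.
; On BeginPlay it flags units with a stealth component in unaware factions as Unaware, and warns if attached to another actor.
; It binds to the grid manager's simulated tile-entry event, broadcasting noise and spot checks at that tile with default ranges through OnMakeNoise and OnCheckIfSeen dispatchers.
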(event Custom|MakeNoise
  (params (Index :type Integer) (Range :type Integer))
  (Default|CallOnMakeNoise Index Range))

(event Custom|AlertUnitsOnEnterTile
  (params (Unit :type BP%20Unit%20Object%20Reference) (GridIndex :type Integer))
  (CallFunction|MakeNoise GridIndex (Variables|Default|GetDefaultNoiseRange))
  (CallFunction|CheckifSeen GridIndex (Variables|Default|GetDefaultSpotRange)))

(event Custom|CheckIfSeen
  (params (Index :type Integer) (Range :type Integer))
  (Default|CallOnCheckifSeen Index Range))

(event EventBeginPlay
  (bind _asbp_grid_manager (Utilities|Casting|CastToBP_GridManager (Components|GetOwner))
    (:then
      (EventDispatchers|BindEventtoOnUnitEnterTileSimulate _asbp_grid_manager (delegate Custom|AlertUnitsOnEnterTile))
      (bind _outactors (Actor|GetAllActorsOfClass "/Game/BattleSystem/Core/Units/BP_Unit.BP_Unit_C"))
      (for _array_element _outactors
        (if (Utilities|Set|Contains (Variables|Default|GetUnawareFactions) (Variables|/Game/BattleSystem/Core/Units/BP_Unit.BP_Unit_C|GetFaction _array_element))
          (if (Utilities|IsValid (Actor|GetComponentbyClass _array_element "/Game/BattleSystem/Core/Units/BP_UnitStealthComponent.BP_UnitStealthComponent_C"))
            (Variables|/Game/BattleSystem/Core/Units/BP_UnitStealthComponent.BP_UnitStealthComponent_C|SetbUnaware (Actor|GetComponentbyClass _array_element "/Game/BattleSystem/Core/Units/BP_UnitStealthComponent.BP_UnitStealthComponent_C") true))))
      (Variables|Default|SetbSetupDone true))
    (:CastFailed
      (Development|PrintString "WARNING: BP_GridManager_StealthSystem added to 
actor other than BP_GridManager" true true "(R=1.000000,G=1.000000,B=0.000000,A=1.000000)"))))