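; BP_GridActor is an actor that occupies a cell on the battle system's grid and tracks its grid index.
; Its construction script finds the BP_GridManager, runs the BPGridAnchor's external construction logic and copies the anchor's index when a manager exists.
; An event and a getter expose the index, with the getter always reporting it valid.
; PlaceActorAtAnchor delegates placement to the anchor.
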(event EventSetGridIndex
  (params (GridIndex :type Integer))
  (Variables|Default|SetGridIndex GridIndex))

(fn ConstructionScript
  (bind _bp_gridanchor (Variables|Default|GetBP_GridAnchor))
  (bind _returnvalue (Actor|GetActorOfClass "/Game/BattleSystem/Core/Grid/BP_GridManager.BP_GridManager_C"))
  (Utilities|IsValid _returnvalue
    (:Is%20Valid
      (Variables|Default|SetGridManagerRef _returnvalue)
      (Default|ExternalConstuctionScript _bp_gridanchor)
      (Variables|Default|SetGridIndex (Variables|/Game/BattleSystem/Core/BP_GridAnchor.BP_GridAnchor_C|GetGridIndex _bp_gridanchor)))))

(fn PlaceActoratAnchor
  (Default|PlaceActoratAnchor (Variables|Default|GetBP_GridAnchor))
  (return))

(fn GetGridIndex
  (return true (Variables|Default|GetGridIndex)))