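; BP_Path_Range is a battle system pathfinding Blueprint that expands a movement range search across the grid one step at a time.
; SearchAndAddAdjacentTiles offsets each open-list tile by the grid manager's BaseEdges to find neighbour indices.
; Indices not yet in Paths are recorded with parent index and parent cost plus one, then returned as the child open list.
; The Move, SearchStep and DelayedSearchTiles inputs are unused here.
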(fn SearchandAddAdjacentTiles
  (params (SearchStep :type Integer%20%28by%20ref%29) (Paths :type Map%20of%20Integers%20to%20Structs) (Move :type Integer%20%28by%20ref%29) (OpenListTiles :type Array%20of%20F%20Pathfinding%20Index%20Structures) (DelayedSearchTiles :type Array%20of%20F%20Pathfinding%20Index%20Structures))
  (for _array_element OpenListTiles
    (for _array_element_2 (Variables|/Game/BattleSystem/Core/Grid/BP_GridManager.BP_GridManager_C|GetBaseEdges (Variables|Default|GetGridManagerRef))
      (if (not (Utilities|Map|Contains Paths (+ _array_element_2 (.index _array_element)))) ; Has the node already been searched (if so the cost should be > 0)
        (Utilities|Map|Add Paths (+ _array_element_2 (.index _array_element)) (Utilities|Struct|MakeFPathfinding (+ (.cost _array_element) 1) (.index _array_element)))
        (Utilities|Array|Add (LocalVariables|GetLocalOpenListChildTiles) (Utilities|Struct|MakeFPathfindingIndex (+ _array_element_2 (.index _array_element)) (+ (.cost _array_element) 1) (.index _array_element))))))
  (return (LocalVariables|GetLocalOpenListChildTiles)))