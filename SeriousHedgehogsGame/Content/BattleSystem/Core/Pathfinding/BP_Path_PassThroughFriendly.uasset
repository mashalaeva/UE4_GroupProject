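; Pathfinding variant for the grid battle system that lets a unit move through tiles occupied by allied units while other units block the way.
; Both run overrides cache the starting unit's allied factions before calling the parent search, and skip the search if the start tile has no unit.
; AddTileIfValid records tiles within move cost and any units on them as reachable, but only expands from empty or allied-occupied tiles.
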(fn AddTileifValid
  (params (EdgeIndex :type Integer%20%28by%20ref%29) (TotalCost :type Integer%20%28by%20ref%29) (ParentIndex :type Integer%20%28by%20ref%29) (Move :type Integer%20%28by%20ref%29) (Paths :type Map%20of%20Integers%20to%20Structs) (OpenListChildTiles :type Array%20of%20F%20Pathfinding%20Index%20Structures))
  (bind _gridmanagerref (Variables|Default|GetGridManagerRef))
  (bind _gridunits (Variables|/Game/BattleSystem/Core/Grid/BP_GridManager.BP_GridManager_C|GetGridUnits _gridmanagerref))
  (bind (_value _returnvalue) (Utilities|Map|Find _gridunits EdgeIndex))
  (if (<= TotalCost Move)
    (Utilities|Map|Add Paths EdgeIndex (Utilities|Struct|MakeFPathfinding TotalCost ParentIndex))
    (if _returnvalue
      (if (Utilities|Set|Contains (Variables|Default|GetPassThroughFactions) (Variables|/Game/BattleSystem/Core/Units/BP_Unit.BP_Unit_C|GetFaction _value))
        (Utilities|Set|Add (Variables|Default|GetReachableUnitIndexes) EdgeIndex)
        (Utilities|Array|Add OpenListChildTiles (Utilities|Struct|MakeFPathfindingIndex EdgeIndex TotalCost ParentIndex) :!label _label)
        (else
          (Utilities|Set|Add (Variables|Default|GetReachableUnitIndexes) EdgeIndex)))
      (else
        (goto _label)))
    (else
      (return))))

(fn RunPathfinding
  (params (StartIndex :type Integer) (MoveRange :type Integer) (GridManager :type BP%20Grid%20Manager%20Object%20Reference))
  (bind _gridunits (Variables|/Game/BattleSystem/Core/Grid/BP_GridManager.BP_GridManager_C|GetGridUnits GridManager))
  (bind (_value _returnvalue) (Utilities|Map|Find _gridunits StartIndex))
  (if _returnvalue
    (Variables|Default|SetPassThroughFactions (Variables|/Game/BattleSystem/Core/Units/BP_Unit.BP_Unit_C|GetAlliedFactions _value))
    (bind (_pathsmap _pathobject) (|CallParentFunction StartIndex MoveRange GridManager))
    (return _pathsmap _pathobject)
    (else
      (return 0 0))))

(fn RunPathfindingUntilIndexFound
  (params (StartIndex :type Integer) (MoveRange :type Integer) (GridManager :type BP%20Grid%20Manager%20Object%20Reference) (TargetGridIndexes :type Array%20of%20Integers))
  (bind _gridunits (Variables|/Game/BattleSystem/Core/Grid/BP_GridManager.BP_GridManager_C|GetGridUnits GridManager))
  (bind (_value _returnvalue) (Utilities|Map|Find _gridunits StartIndex))
  (if _returnvalue
    (Variables|Default|SetPassThroughFactions (Variables|/Game/BattleSystem/Core/Units/BP_Unit.BP_Unit_C|GetAlliedFactions _value))
    (bind (_bfoundatleastone _foundgridindexes _pathsmap _pathobject) (|CallParentFunction StartIndex MoveRange GridManager TargetGridIndexes))
    (return _bfoundatleastone _foundgridindexes _pathsmap _pathobject)))