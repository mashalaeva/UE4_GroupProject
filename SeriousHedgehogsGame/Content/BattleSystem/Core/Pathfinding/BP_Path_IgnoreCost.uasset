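; Grid pathfinding variant for the battle system that expands a search frontier without checking movement cost.
; SearchAndAddAdjacentTiles walks each open tile's edges in GridManager and passes unvisited neighbours to AddTileIfValid, returning the next frontier.
; AddTileIfValid records every neighbour with its parent and a non-accumulated edge cost plus one, ignoring the Move budget.
; Occupied tiles are logged as reachable units and excluded from further expansion.
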(fn SearchandAddAdjacentTiles
  (params (SearchStep :type Integer%20%28by%20ref%29) (Paths :type Map%20of%20Integers%20to%20Structs) (Move :type Integer%20%28by%20ref%29) (OpenListTiles :type Array%20of%20F%20Pathfinding%20Index%20Structures) (DelayedSearchTiles :type Array%20of%20F%20Pathfinding%20Index%20Structures))
  (if (< (LocalVariables|GetLocalOpenListIndex) (Utilities|Array|Length OpenListTiles)) :!label _label
    (Utilities|FlowControl|Sequence
      (:then_0
        (bind _output_get (LocalVariables|SetLocalEdges (.edges (.Value (Utilities|Map|Find (Variables|/Game/BattleSystem/Core/Grid/BP_GridManager.BP_GridManager_C|GetGridEdges (Variables|Default|GetGridManagerRef)) (.index (Utilities|Array|Get(acopy) OpenListTiles (LocalVariables|GetLocalOpenListIndex))))))))
        (bind _keys (Utilities|Map|Keys _output_get))
        (LocalVariables|SetLocalEdgesIndex 0)
        (if (< (LocalVariables|GetLocalEdgesIndex) (Utilities|Array|Length _keys)) :!label _label_2
          (if (Utilities|Map|Contains Paths (Utilities|Array|Get(acopy) _keys (LocalVariables|GetLocalEdgesIndex)))
            _
            (else
              (CallFunction|AddTileifValid (Utilities|Array|Get(acopy) _keys (LocalVariables|GetLocalEdgesIndex)) (+ (.Value (Utilities|Map|Find (LocalVariables|GetLocalEdges) (Utilities|Array|Get(acopy) _keys (LocalVariables|GetLocalEdgesIndex)))) 1) (.index (Utilities|Array|Get(acopy) OpenListTiles (LocalVariables|GetLocalOpenListIndex))) Move Paths (LocalVariables|GetLocalOpenListChildTiles))))
          (LocalVariables|SetLocalEdgesIndex (+ (LocalVariables|GetLocalEdgesIndex) 1))
          (goto _label_2)))
      (:then_1
        (LocalVariables|SetLocalOpenListIndex (+ (LocalVariables|GetLocalOpenListIndex) 1))
        (goto _label)))
    (else
      (return (LocalVariables|GetLocalOpenListChildTiles)))))

(fn AddTileifValid
  (params (EdgeIndex :type Integer%20%28by%20ref%29) (TotalCost :type Integer%20%28by%20ref%29) (ParentIndex :type Integer%20%28by%20ref%29) (Move :type Integer%20%28by%20ref%29) (Paths :type Map%20of%20Integers%20to%20Structs) (OpenListChildTiles :type Array%20of%20F%20Pathfinding%20Index%20Structures))
  (Utilities|Map|Add Paths EdgeIndex (Utilities|Struct|MakeFPathfinding TotalCost ParentIndex))
  (if (Utilities|Map|Contains (Variables|/Game/BattleSystem/Core/Grid/BP_GridManager.BP_GridManager_C|GetGridUnits (Variables|Default|GetGridManagerRef)) EdgeIndex)
    (Utilities|Set|Add (Variables|Default|GetReachableUnitIndexes) EdgeIndex)
    (else
      (Utilities|Array|Add OpenListChildTiles (Utilities|Struct|MakeFPathfindingIndex EdgeIndex TotalCost ParentIndex))))
  (return))