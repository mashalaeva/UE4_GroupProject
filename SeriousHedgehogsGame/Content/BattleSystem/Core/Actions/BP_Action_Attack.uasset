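; BP_Action_Attack is a battle action that plays the source puppet's attack animation toward the target puppet's location.
; If the source has a BP_PuppetComponent, it binds to that component's animation event, then unbinds and ends the action when the event fires.
; Without that component, it still sends the animation message but ends the action immediately.
; The graph itself applies no damage or other effect.
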(event Custom|AttackHit
  (params (AnimatingActor :type Actor%20Object%20Reference) (Animation :type Gameplay%20Tag%20Structure))
  (EventDispatchers|UnbindEventfromOnAnimationEvent (Actor|GetComponentbyClass (Variables|Default|GetSourcePuppet) "/Game/BattleSystem/Core/Units/BP_PuppetComponent.BP_PuppetComponent_C") (delegate Custom|AttackHit))
  (CallFunction|EndAction true))

(event EventPlayAction
  (bind _sourcepuppet (Variables|Default|GetSourcePuppet))
  (bind _returnvalue (Actor|GetComponentbyClass _sourcepuppet "/Game/BattleSystem/Core/Units/BP_PuppetComponent.BP_PuppetComponent_C"))
  (Utilities|IsValid _returnvalue
    (:Is%20Valid
      (EventDispatchers|BindEventtoOnAnimationEvent _returnvalue (delegate Custom|AttackHit))
      (Class|BPIPuppet|AnimatePuppet(Message) (Variables|Default|GetSourcePuppet) "(TagName=\"Anim.Attack\")" (Transformation|GetActorLocation (Variables|Default|GetTargetPuppet)) :!label _label))
    (:Is%20Not%20Valid
      (Utilities|FlowControl|Sequence
        (:then_0
          (goto _label))
        (:then_1
          (CallFunction|EndAction true))))))

(fn ConstructionScript
  (|CallParentFunction))