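; Battle system action that tells a puppet actor to play an animation, passing along a location.
; It sends the AnimatePuppet message, then either ends immediately or, if set to wait, binds to the puppet component's animation-end event.
; The waiting action unbinds and ends once the matching animation finishes, and also ends right away if the puppet has no puppet component.
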(event Custom|EndAfterAnim
  (params (AnimatingActor :type Actor%20Object%20Reference) (Animation :type Gameplay%20Tag%20Structure))
  (if (== Animation (Variables|Default|GetAnimation))
    (EventDispatchers|UnbindEventfromOnAnimationEnd (Actor|GetComponentbyClass (Variables|Default|GetPuppet) "/Game/BattleSystem/Core/Units/BP_PuppetComponent.BP_PuppetComponent_C") (delegate Custom|EndAfterAnim))
    (CallFunction|EndAction true)))

(event EventPlayAction
  (bind _puppet (Variables|Default|GetPuppet))
  (bind _returnvalue (Actor|GetComponentbyClass _puppet "/Game/BattleSystem/Core/Units/BP_PuppetComponent.BP_PuppetComponent_C"))
  (Class|BPIPuppet|AnimatePuppet(Message) (Variables|Default|GetPuppet) (Variables|Default|GetAnimation) (Variables|Default|GetLocation))
  (if (Variables|Default|GetbWaitForAnimEnd)
    (if (Utilities|IsValid _returnvalue)
      (EventDispatchers|BindEventtoOnAnimationEnd _returnvalue (delegate Custom|EndAfterAnim))
      (else
        (CallFunction|EndAction true :!label _label)))
    (else
      (goto _label))))

(fn ConstructionScript
  (|CallParentFunction))