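; BP_StatusEffect_Woke is a battle status effect, apparently marking a unit as woken, that lasts until turn start.
; On activation it queues a grid camera pan to the target unit's puppet, runs the parent activation, then queues a discovery sound at the owning unit's puppet.
; At turn start it queues its own removal.
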(event EventActivate
  (params (Target%20Unit :type BP%20Unit%20Object%20Reference))
  (Default|QueuePanCamera (.GridCamera (CallFunction|GetGridCamera)) (Transformation|GetActorLocation (Variables|/Game/BattleSystem/Core/Units/BP_Unit.BP_Unit_C|GetPuppet Target%20Unit)) 0 1.0)
  (|CallParentFunction Target%20Unit)
  (Default|QueuePlaySound (.ActionManager (CallFunction|GetActionManager)) "/Game/BattleSystem/Core/Abilities/A_Discover.A_Discover" (Transformation|GetActorLocation (Variables|/Game/BattleSystem/Core/Units/BP_Unit.BP_Unit_C|GetPuppet (Variables|Default|GetOwningUnit))) 1.0 1.0 0.0 0 0 1.0))

(event EventRunonTurnStart
  (CallFunction|QueueRemoveStatusEffect))

(fn ConstructionScript
  (|CallParentFunction))