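; BP_StatusEffect is a base actor for status effects on units in the grid battle system, with empty turn-start and turn-end hooks.
; Activate registers it in the target's BP_AbilitySystem StatusEffects list and stores the owning unit, warning if that component is missing.
; Disable removes it from that list.
; When an icon is set, both spawn BP_Action_DisplayStatusEffect actors to show or remove the effect on the unit's puppet.
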(event Custom|RunOnTurnEnd)

(event Custom|RunOnTurnStart)

(event Custom|Activate
  (params (Target%20Unit :type BP%20Unit%20Object%20Reference))
  (bind _returnvalue (Actor|GetComponentbyClass Target%20Unit "/Game/BattleSystem/Core/Units/BP_AbilitySystem.BP_AbilitySystem_C"))
  (if (Utilities|IsValid _returnvalue)
    (Utilities|Array|Add (Variables|/Game/BattleSystem/Core/Units/BP_AbilitySystem.BP_AbilitySystem_C|GetStatusEffects _returnvalue) self)
    (Variables|Default|SetOwningUnit Target%20Unit)
    (CallFunction|QueueAddStatusEffect)
    (else
      (Development|PrintString "WARNING: Attempted to activate status effect on unit without ability system component" true true "(R=1.000000,G=1.000000,B=0.000000,A=1.000000)"))))

(event Custom|Disable
  (Utilities|FlowControl|Sequence
    (:then_0
      (bind _owningunit (Variables|Default|GetOwningUnit)
        (:then
          (if (Utilities|IsValid (Actor|GetComponentbyClass _owningunit "/Game/BattleSystem/Core/Units/BP_AbilitySystem.BP_AbilitySystem_C"))
            (Utilities|Array|RemoveItem (Variables|/Game/BattleSystem/Core/Units/BP_AbilitySystem.BP_AbilitySystem_C|GetStatusEffects (Actor|GetComponentbyClass _owningunit "/Game/BattleSystem/Core/Units/BP_AbilitySystem.BP_AbilitySystem_C")) self)))
        (:else)))
    (:then_1
      (CallFunction|QueueRemoveStatusEffect))))

(event EventBeginPlay
  (Variables|Default|SetGridManagerRef (.GridManager (CallFunction|GetGridManager))))

(fn ConstructionScript)

(fn QueueAddStatusEffect
  (Utilities|IsValid (Variables|Default|GetEffectIcon)
    (:Is%20Valid
      (Game|SpawnActorfromClass "/Game/BattleSystem/Core/Actions/BP_Action_DisplayStatusEffect.BP_Action_DisplayStatusEffect_C" (Math|Transform|MakeTransform "0, 0, 0" "0, 0, 0" "1,1,1") "AlwaysSpawn" 0 (Variables|/Game/BattleSystem/Core/Units/BP_Unit.BP_Unit_C|GetPuppet (Variables|Default|GetOwningUnit)) (Utilities|GetClass self) false -1.0 "NewEnumerator0" 0)
      (return))))

(fn QueueRemoveStatusEffect
  (Utilities|IsValid (Variables|Default|GetEffectIcon)
    (:Is%20Valid
      (Game|SpawnActorfromClass "/Game/BattleSystem/Core/Actions/BP_Action_DisplayStatusEffect.BP_Action_DisplayStatusEffect_C" (Math|Transform|MakeTransform "0, 0, 0" "0, 0, 0" "1,1,1") "Undefined" 0 (Variables|/Game/BattleSystem/Core/Units/BP_Unit.BP_Unit_C|GetPuppet (Variables|Default|GetOwningUnit)) (Utilities|GetClass self) true -1.0 "NewEnumerator0" 0)
      (return))))