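; Unit component for the grid stealth system that keeps an enemy or other unit unaware until it spots or hears something.
; On BeginPlay it waits for the grid manager's stealth system to finish setup, then binds Spot and Listen to its sight and noise events.
; Spot requires facing, range, tile visibility and, with a cover system, a clear trace; Listen checks tile distance.
; Waking adds a Woke status, moves initiative and unbinds alerts.
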(event Custom|UnbindAlertEvents
  ;[0 0 0] Setup
  (EventDispatchers|UnbindEventfromOnCheckifSeen (Actor|GetComponentbyClass (stale EventBeginPlay _output_get) "/Game/BattleSystem/Core/Grid/BP_StealthSystem.BP_StealthSystem_C") (delegate Custom|Spot))
  (EventDispatchers|UnbindEventfromOnMakeNoise (Actor|GetComponentbyClass (stale EventBeginPlay _output_get) "/Game/BattleSystem/Core/Grid/BP_StealthSystem.BP_StealthSystem_C") (delegate Custom|Listen)))

(event Custom|Wake
  (bind _owningunit (Variables|Default|GetOwningUnit))
  (bind _returnvalue (Actor|GetComponentbyClass _owningunit "/Game/BattleSystem/Core/Units/BP_AbilitySystem.BP_AbilitySystem_C"))
  ;[0 0 0] Wake
  (if (and (Variables|Default|GetbUnaware) (not (Variables|Default|GetbCannotWake)))
    (Variables|Default|SetbUnaware false)
    (if (Utilities|Map|Contains (Variables|/Game/BattleSystem/Core/Grid/BP_GridManager.BP_GridManager_C|GetGridUnits (Variables|Default|GetGridManagerRef)) (Variables|/Game/BattleSystem/Core/Units/BP_Unit.BP_Unit_C|GetGridIndex (Variables|Default|GetOwningUnit)))
      (if (Utilities|IsValid _returnvalue)
        (Default|AddStatusEffect _returnvalue "/Game/BattleSystem/Core/Abilities/BP_StatusEffect_Woke.BP_StatusEffect_Woke_C"))
      (Default|MoveActorinInitiative (.TurnManager (CallFunction|GetTurnManager)) (Variables|Default|GetInitiativeOnWake) (Variables|Default|GetOwningUnit))
      (CallFunction|UnbindAlertEvents))))

(event Custom|Spot
  (params (Index :type Integer) (Range :type Integer))
  (bind _gridmanagerref (Variables|Default|GetGridManagerRef))
  (bind _gridmanagerref_2 (Variables|Default|GetGridManagerRef))
  (bind _gridmanagerref_3 (Variables|Default|GetGridManagerRef))
  (bind _owningunit (Variables|Default|GetOwningUnit))
  (bind _gridlocations (Variables|/Game/BattleSystem/Core/Grid/BP_GridManager.BP_GridManager_C|GetGridLocations _gridmanagerref_3))
  (bind _gridindex (Variables|/Game/BattleSystem/Core/Units/BP_Unit.BP_Unit_C|GetGridIndex _owningunit))
  (bind _distance (Default|FindDistanceIinTilesBetweenIndexes _gridmanagerref _gridindex Index false))
  ;[0 0 0] Spot
  (if (Variables|Default|GetbUnaware)
    (if (>= (Math|Vector|DotProduct (Transformation|GetActorForwardVector (Variables|/Game/BattleSystem/Core/Units/BP_Unit.BP_Unit_C|GetPuppet (Variables|Default|GetOwningUnit))) (- (.Value (Utilities|Map|Find _gridlocations Index)) (.Value (Utilities|Map|Find _gridlocations (Variables|/Game/BattleSystem/Core/Units/BP_Unit.BP_Unit_C|GetGridIndex (Variables|Default|GetOwningUnit)))))) -0.01)
      (if (>= Range _distance)
        (bind _bvisible (Default|CheckifTileIsVisiblefromOtherTile (Variables|Default|GetGridManagerRef) (Variables|/Game/BattleSystem/Core/Units/BP_Unit.BP_Unit_C|GetGridIndex (Variables|Default|GetOwningUnit)) Index (* _distance (Variables|/Game/BattleSystem/Core/Grid/BP_GridManager.BP_GridManager_C|GetTileXSize (Variables|Default|GetGridManagerRef))) 0 true false))
        (if _bvisible
          (if (Utilities|IsValid (Actor|GetComponentbyClass (Variables|Default|GetGridManagerRef) "/Game/BattleSystem/Core/Grid/BP_CoverSystem.BP_CoverSystem_C"))
            (bind _hit (Default|TraceonGrid _gridmanagerref_2 (Variables|/Game/BattleSystem/Core/Units/BP_Unit.BP_Unit_C|GetGridIndex (Variables|Default|GetOwningUnit)) Index "TraceTypeQuery5" "None" (Variables|/Game/BattleSystem/Core/Grid/BP_GridManager.BP_GridManager_C|GetVisibilityTraceHeight _gridmanagerref_2)))
            (if (not _hit)
              (CallFunction|Wake :!label _label))
            (else
              (goto _label))))))))

(event Custom|Listen
  (params (Index :type Integer) (Range :type Integer))
  ;[0 0 0] Listen
  (if (Variables|Default|GetbUnaware)
    (if (>= Range (Default|FindDistanceIinTilesBetweenIndexes (Variables|Default|GetGridManagerRef) Index (Variables|/Game/BattleSystem/Core/Units/BP_Unit.BP_Unit_C|GetGridIndex (Variables|Default|GetOwningUnit)) false))
      (CallFunction|Wake))))

(event EventBeginPlay
  (bind (_bvalid _gridmanager) (CallFunction|GetGridManager))
  ;[0 0 0] Setup
  (bind _asbp_unit (Utilities|Casting|CastToBP_Unit (Components|GetOwner))
    (:then
      (Variables|Default|SetOwningUnit _asbp_unit)
      (if _bvalid
        (bind _output_get (Variables|Default|SetGridManagerRef _gridmanager))
        (if (Utilities|IsValid (Actor|GetComponentbyClass _output_get "/Game/BattleSystem/Core/Grid/BP_StealthSystem.BP_StealthSystem_C"))
          (if (Variables|/Game/BattleSystem/Core/Grid/BP_StealthSystem.BP_StealthSystem_C|GetbSetupDone (Actor|GetComponentbyClass _output_get "/Game/BattleSystem/Core/Grid/BP_StealthSystem.BP_StealthSystem_C")) :!label _label
            (if (Variables|Default|GetbUnaware)
              (if (Variables|Default|GetbCanSpot)
                (EventDispatchers|BindEventtoOnCheckifSeen (Actor|GetComponentbyClass _output_get "/Game/BattleSystem/Core/Grid/BP_StealthSystem.BP_StealthSystem_C") (delegate Custom|Spot)))
              (if (Variables|Default|GetbCanListen)
                (EventDispatchers|BindEventtoOnMakeNoise (Actor|GetComponentbyClass _output_get "/Game/BattleSystem/Core/Grid/BP_StealthSystem.BP_StealthSystem_C") (delegate Custom|Listen))))
            (else
              (Utilities|FlowControl|Delay 0.0)
              (goto _label)))
          (else
            (Development|PrintString "WARNING: Unit has stealth system, but Grid Manager does not." true true "(R=1.000000,G=1.000000,B=0.000000,A=1.000000)")))))
    (:CastFailed
      (Development|PrintString "WARNING: BP_Unit_StealthSystem added to 
actor other than BP_Unit" true true "(R=1.000000,G=1.000000,B=0.000000,A=1.000000)"))))